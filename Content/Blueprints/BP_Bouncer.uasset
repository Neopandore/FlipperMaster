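; Pinball-style bouncer actor that kicks out along its local Y axis when a BP_FlipperBall overlaps its Box.
; BeginPlay finds the target position by briefly teleporting by Offset and back, storing both locations.
; The Bounce timeline interpolates between them with a swept move, then reverses on finish.
; A DoOnce blocks retriggering until the reverse starts.
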(event `self.ReceiveBeginPlay`
  (set `self.InitialLocation` (`self.K2_GetActorLocation`))
  (`self.K2_AddActorLocalOffset` (`KismetMathLibrary.MakeVector` 0.0 (`self.Offset`)) false true)
  (set `self.UpdatedLocation` (`self.K2_GetActorLocation`))
  (`self.K2_SetActorLocation` (`self.InitialLocation`) false true))

(event `self.Box.OnComponentBeginOverlap`
  (params (OverlappedComponent :type "PrimitiveComponent Object Reference") (OtherActor :type "Actor Object Reference") (OtherComp :type "PrimitiveComponent Object Reference") (OtherBodyIndex :type Integer) (bFromSweep :type Boolean) (SweepResult :type "HitResult Structure (by ref)"))
  (bind _initiallocation (`self.InitialLocation`))
  (cast `/Game/Blueprints/BP_FlipperBall` OtherActor)
  (`/Engine/EditorBlueprintResources/StandardMacros.DoOnce` false :!label _label
    (:`Completed`
      (bind (_direction _offset) (`Timeline|Bounce` :!label _label_2)
        (:`Update`
          (`self.K2_SetActorLocation` (- _initiallocation (* (- _initiallocation (`self.UpdatedLocation`)) _offset)) true))
        (:`Finished`
          (`self.Reverse`))))))

(event `Reverse`
  (`|ExecutionSequence`
    (:`then_0`
      (goto _label_2 :!via `Reverse`))
    (:`then_1`
      (goto _label :!via `Reset`))))

(fn `UserConstructionScript`)