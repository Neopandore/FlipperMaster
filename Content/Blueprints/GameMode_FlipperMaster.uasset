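; Game mode for a flipper game that tracks score and the persistent best score, and opens the HUD and menu widgets.
; BeginPlay shows the game menu and in-game HUD, then copies the best score from the "BestScore" save slot into GameInstance_Flipper.
; AddScore adds multiplier-scaled points, and PauseGame shows the pause menu.
; EndGame saves any new record through a save object created at BeginPlay, then shows the end menu.
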(event `self.ReceiveBeginPlay`
  (`WidgetBlueprintLibrary.SetFocusToGameViewport`)
  (`KismetSystemLibrary.Delay` 0.1)
  (bind _returnvalue (`|CreateWidget` "/Game/UMG/HUD_GameMenu.HUD_GameMenu_C"))
  (`UserWidget.AddToViewport` _returnvalue 0)
  (bind _returnvalue_2 (`|CreateWidget` "/Game/UMG/HUD_InGame.HUD_InGame_C"))
  (`UserWidget.AddToViewport` _returnvalue_2 0)
  (bind _returnvalue_3 (`GameplayStatics.CreateSaveGameObject` "/Game/Blueprints/BestScore_Save.BestScore_Save_C"))
  (set `self.Save_Ref` _returnvalue_3)
  (bind _returnvalue_4 (`GameplayStatics.LoadGameFromSlot` "BestScore"))
  (bind _asbest_score_save (cast `/Game/Blueprints/BestScore_Save` _returnvalue_4))
  (bind _asgame_instance_flipper (cast `/Game/Blueprints/GameInstance_Flipper` (`GameplayStatics.GetGameInstance`)))
  (set `/Game/Blueprints/GameInstance_Flipper.BestScore` (`/Game/Blueprints/BestScore_Save.BestScore_Save` _asbest_score_save) _asgame_instance_flipper))

(event `AddScore`
  (params (ScoreValue :type Integer))
  (set `self.Score` (+ (`self.Score`) (* ScoreValue (`self.Multiplier`)))))

(event `EndGame`
  (bind _save_ref (`self.Save_Ref`))
  (bind _score (`self.Score`))
  (bind _asgame_instance_flipper (cast `/Game/Blueprints/GameInstance_Flipper` (`GameplayStatics.GetGameInstance`)))
  (if (> _score (`/Game/Blueprints/GameInstance_Flipper.BestScore` _asgame_instance_flipper))
    (bind _output_get (set `/Game/Blueprints/GameInstance_Flipper.BestScore` _score _asgame_instance_flipper))
    (set `/Game/Blueprints/BestScore_Save.BestScore_Save` _output_get _save_ref)
    (`GameplayStatics.SaveGameToSlot` _save_ref "BestScore")
    (`KismetSystemLibrary.Delay` 1.0))
  (bind _returnvalue (`|CreateWidget` "/Game/UMG/HUD_EndMenu.HUD_EndMenu_C"))
  (`UserWidget.AddToViewport` _returnvalue 0))

(event `PauseGame`
  (bind _returnvalue (`|CreateWidget` "/Game/UMG/HUD_PauseMenu.HUD_PauseMenu_C"))
  (`UserWidget.AddToViewport` _returnvalue 0))

(fn `UserConstructionScript`)