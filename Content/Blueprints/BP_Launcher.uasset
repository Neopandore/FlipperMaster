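; Launcher actor that is pulled back while pressed and driven by a timeline on release, like a plunger.
; IPress stops the Launch timeline and starts a looping timer that nudges the root along negative local X with sweep, up to a fixed travel limit.
; IRelease clears the timer and plays Launch, whose LocationPercent positions the actor between its pulled and initial locations with a swept move.
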(event `self.ReceiveBeginPlay`
  (set `self.InitLocation` (`self.K2_GetActorLocation`)))

(event `/Game/Blueprints/iFlipperTrigger.iPress`
  (set `self.UpdatedLocation` (`self.K2_GetActorLocation`))
  (bind _returnvalue (`KismetSystemLibrary.K2_SetTimerDelegate` (delegate `AddOffset`) (`GameplayStatics.GetWorldDeltaSeconds`) true))
  (set `self.OffsetTimer` _returnvalue)
  (`self.StopLauncher`))

(event `AddOffset`
  (bind _initlocation_x (`KismetMathLibrary.BreakVector` (`self.InitLocation`)))
  (bind _updatedlocation_x (`KismetMathLibrary.BreakVector` (`self.UpdatedLocation`)))
  (if (< (`KismetMathLibrary.Abs` (- _initlocation_x _updatedlocation_x)) 200.0)
    (`SceneComponent.K2_AddLocalOffset` (`self.DefaultSceneRoot`) (-0.1 0.0 0.0) true false)
    (set `self.UpdatedLocation` (`self.K2_GetActorLocation`))))

(event `/Game/Blueprints/iFlipperTrigger.iRelease`
  (bind _initlocation (`self.InitLocation`))
  (`KismetSystemLibrary.K2_ClearAndInvalidateTimerHandle` (`self.OffsetTimer`))
  (bind (_direction _locationpercent) (`Timeline|Launch` :!via `PlayFromStart` :!label _label)
    (:`Update`
      (`self.K2_SetActorLocation` (- _initlocation (* (- _initlocation (`self.UpdatedLocation`)) _locationpercent)) true))
    (:`Finished`
      (set `self.UpdatedLocation` (`self.K2_GetActorLocation`)))))

(event `StopLauncher`
  (goto _label :!via `Stop`))

(fn `UserConstructionScript`)