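; BP_FlipperBall is the pinball ball actor, which drives scoring from what it collides with.
; On hit, it ignores the launcher and the game mode's table and blocking objects.
; IPoints objects add the ball's score value, and both they and IFlipperTrigger objects raise the GameMode_FlipperMaster multiplier and play an explosion sound.
; Any other hit resets the multiplier to one.
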(event `self.ReceiveBeginPlay`
  (bind _asgame_mode_flipper_master (cast `/Game/Blueprints/GameMode_FlipperMaster` (`GameplayStatics.GetGameMode`)))
  (set `self.Gamemode_Ref` _asgame_mode_flipper_master))

(event `self.ReceiveHit`
  (params (MyComp :type "PrimitiveComponent Object Reference") (Other :type "Actor Object Reference") (OtherComp :type "PrimitiveComponent Object Reference") (bSelfMoved :type Boolean) (HitLocation :type "Vector Structure") (HitNormal :type "Vector Structure") (NormalImpulse :type "Vector Structure") (Hit :type "HitResult Structure (by ref)"))
  (bind _gamemode_ref (`self.Gamemode_Ref`))
  (cast `/Game/Blueprints/BP_Launcher` Other
    (:`CastFailed`
      (if (or (== Other (`/Game/Blueprints/GameMode_FlipperMaster.Table` _gamemode_ref)) (== Other (`/Game/Blueprints/GameMode_FlipperMaster.Blocking` _gamemode_ref)))
        _
        (elif (`KismetSystemLibrary.DoesImplementInterface` Other "/Game/Blueprints/iPoints.iPoints_C")
          (`/Game/Blueprints/GameMode_FlipperMaster.AddScore` _gamemode_ref (`self.ScoreValue`))
          (set `/Game/Blueprints/GameMode_FlipperMaster.Multiplier` (+ (`/Game/Blueprints/GameMode_FlipperMaster.Multiplier` _gamemode_ref) 1) _gamemode_ref)
          (`GameplayStatics.PlaySoundAtLocation` "/Game/StarterContent/Audio/Explosion01.Explosion01" HitLocation :!label _label)
          (elif (`KismetSystemLibrary.DoesImplementInterface` Other "/Game/Blueprints/iFlipperTrigger.iFlipperTrigger_C")
            (set `/Game/Blueprints/GameMode_FlipperMaster.Multiplier` (+ (`/Game/Blueprints/GameMode_FlipperMaster.Multiplier` _gamemode_ref) 1) _gamemode_ref)
            (goto _label)
            (else
              (set `/Game/Blueprints/GameMode_FlipperMaster.Multiplier` 1 _gamemode_ref))))))))

(fn `UserConstructionScript`)