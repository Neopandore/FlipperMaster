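; Pinball target that pulses in size and fires a radial impulse when hit by a BP_FlipperBall.
; On a hit, the Scale timeline scales the actor's X and Y from its starting size, keeps Z fixed, then plays in reverse on finish.
; It also sets the RadialForce component's ForceStrength from the FlipperMaster game mode's Multiplier before calling FireImpulse.
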(event `self.ReceiveBeginPlay`
  (set `self.InitialTranform` (`self.GetActorScale3D`))
  (bind _asgame_mode_flipper_master (cast `/Game/Blueprints/GameMode_FlipperMaster` (`GameplayStatics.GetGameMode`)))
  (set `self.GameMode_Ref` _asgame_mode_flipper_master))

(event `self.ReceiveHit`
  (params (MyComp :type "PrimitiveComponent Object Reference") (Other :type "Actor Object Reference") (OtherComp :type "PrimitiveComponent Object Reference") (bSelfMoved :type Boolean) (HitLocation :type "Vector Structure") (HitNormal :type "Vector Structure") (NormalImpulse :type "Vector Structure") (Hit :type "HitResult Structure (by ref)"))
  (cast `/Game/Blueprints/BP_FlipperBall` Other)
  (`self.Animate`)
  (set `RadialForceComponent.ForceStrength` (`KismetMathLibrary.Conv_IntToDouble` (`/Game/Blueprints/GameMode_FlipperMaster.Multiplier` (`self.GameMode_Ref`))) (`self.RadialForce`))
  (`RadialForceComponent.FireImpulse` (`self.RadialForce`)))

(event `Animate`
  (bind (_initialtranform_x _initialtranform_y _initialtranform_z) (`KismetMathLibrary.BreakVector` (`self.InitialTranform`)))
  (bind (_direction _scale_up) (`Timeline|Scale` :!label _label)
    (:`Update`
      (bind (_returnvalue_x _returnvalue_y) (`KismetMathLibrary.BreakVector` (* (`KismetMathLibrary.MakeVector` _initialtranform_x _initialtranform_y) _scale_up)))
      (`self.SetActorScale3D` (`KismetMathLibrary.MakeVector` _returnvalue_x _returnvalue_y _initialtranform_z)))
    (:`Finished`
      (`self.Reverse`))))

(event `Reverse`
  (goto _label :!via `Reverse`))

(fn `UserConstructionScript`)