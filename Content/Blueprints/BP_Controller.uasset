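; BP_Controller is the input controller for a pinball game, routing player input to the flippers and launcher.
; On BeginPlay it finds actors implementing IFlipperTrigger and casts them to cache the left flipper, right flipper and launcher.
; The Left, Right and Other input actions forward press and release as interface messages to those cached actors.
; Escape calls PauseGame on GameMode_FlipperMaster.
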(event `self.ReceiveBeginPlay`
  (bind _outactors (`GameplayStatics.GetAllActorsWithInterface` "/Game/Blueprints/iFlipperTrigger.iFlipperTrigger_C"))
  (for _array_element _outactors
    (bind _asbp_flipper_left (cast `/Game/Blueprints/BP_FlipperLeft` _array_element)
      (:`then`
        (set `self.Flipper_Left` _asbp_flipper_left))
      (:`CastFailed`
        (bind _asbp_flipper_right (cast `/Game/Blueprints/BP_FlipperRight` _array_element)
          (:`then`
            (set `self.Flipper_Right` _asbp_flipper_right))
          (:`CastFailed`
            (bind _asbp_launcher (cast `/Game/Blueprints/BP_Launcher` _array_element))
            (set `self.Launcher` _asbp_launcher)))))))

(event `InputAction|Left`
  (params (Key :type "Key Structure" :default "AnyKey"))
  (bind _flipper_left (`self.Flipper_Left`))
  (:`Pressed`
    (message `/Game/Blueprints/iFlipperTrigger.iPress` _flipper_left))
  (:`Released`
    (message `/Game/Blueprints/iFlipperTrigger.iRelease` _flipper_left)))

(event `InputAction|Right`
  (params (Key :type "Key Structure" :default "AnyKey"))
  (bind _flipper_right (`self.Flipper_Right`))
  (:`Pressed`
    (message `/Game/Blueprints/iFlipperTrigger.iPress` _flipper_right))
  (:`Released`
    (message `/Game/Blueprints/iFlipperTrigger.iRelease` _flipper_right)))

(event `InputAction|Other`
  (params (Key :type "Key Structure" :default "AnyKey"))
  (bind _launcher (`self.Launcher`))
  (:`Pressed`
    (message `/Game/Blueprints/iFlipperTrigger.iPress` _launcher))
  (:`Released`
    (message `/Game/Blueprints/iFlipperTrigger.iRelease` _launcher)))

(event `Key|Escape` :paused true
  (params (Key :type "Key Structure" :default "AnyKey"))
  (:`Pressed`
    (bind _asgame_mode_flipper_master (cast `/Game/Blueprints/GameMode_FlipperMaster` (`GameplayStatics.GetGameMode`)))
    (`/Game/Blueprints/GameMode_FlipperMaster.PauseGame` _asgame_mode_flipper_master)))

(fn `UserConstructionScript`)